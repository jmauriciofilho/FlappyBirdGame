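; FloorActor is a scrolling floor actor that slides along the world X axis and loops.
; Each Tick offsets it by Speed scaled by DeltaSeconds, without sweeping.
; Once its absolute X position reaches Width, it snaps back to X zero while keeping Y and Z, producing a repeating treadmill-style motion.
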(event `self.ReceiveTick`
  (params (DeltaSeconds :type "Float (single-precision)"))
  (`self.K2_AddActorWorldOffset` (`KismetMathLibrary.MakeVector` (* DeltaSeconds (`self.Speed`))))
  (if (>= (`KismetMathLibrary.Abs` (.x (`self.K2_GetActorLocation`))) (`self.Width`))
    (`self.K2_SetActorLocation` (`KismetMathLibrary.MakeVector` 0.0 (.y (`self.K2_GetActorLocation`)) (.z (`self.K2_GetActorLocation`))))))

(fn `UserConstructionScript`)